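; BP_Apple is a falling collectible that resolves as either caught or missed in an apple-catching game.
; A hit on its Sphere by BP_Bucket plays a success sound and fires OnAppleCollected on BP_GameState.
; An overlap with BP_DeadZone plays a failure sound and fires OnAppleFalled on the same game state.
; Either outcome destroys the apple, leaving any further consequences to the game state.
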(event `self.Sphere.OnComponentHit`
  (params (HitComponent :type "PrimitiveComponent Object Reference") (OtherActor :type "Actor Object Reference") (OtherComp :type "PrimitiveComponent Object Reference") (NormalImpulse :type "Vector Structure") (Hit :type "HitResult Structure (by ref)"))
  ;[1 1 1] Bucket collision handling
  (cast `/Game/Blueprints/BP_Bucket` OtherActor)
  (`|ExecutionSequence`
    (:`then_0`
      (`GameplayStatics.PlaySound2D` "/Engine/EditorSounds/Notifications/CompileSuccess.CompileSuccess" 1.0 1.0 0.0 null null))
    (:`then_1`
      (bind _asbp_game_state (cast `/Game/GameSettings/BP_GameState` (`GameplayStatics.GetGameState`)))
      (`/Game/GameSettings/BP_GameState.OnAppleCollected` _asbp_game_state))
    (:`then_2`
      (`self.K2_DestroyActor`))))

(event `self.Sphere.OnComponentBeginOverlap`
  (params (OverlappedComponent :type "PrimitiveComponent Object Reference") (OtherActor :type "Actor Object Reference") (OtherComp :type "PrimitiveComponent Object Reference") (OtherBodyIndex :type Integer) (bFromSweep :type Boolean) (SweepResult :type "HitResult Structure (by ref)"))
  ;[1 1 1] DeadZone collision handling
  (cast `/Game/Blueprints/BP_DeadZone` OtherActor)
  (`|ExecutionSequence`
    (:`then_0`
      (`GameplayStatics.PlaySound2D` "/Engine/EditorSounds/Notifications/CompileFailed.CompileFailed" 1.0 1.0 0.0 null null))
    (:`then_1`
      (bind _asbp_game_state (cast `/Game/GameSettings/BP_GameState` (`GameplayStatics.GetGameState`)))
      (`/Game/GameSettings/BP_GameState.OnAppleFalled` _asbp_game_state))
    (:`then_2`
      (`self.K2_DestroyActor`))))

(fn `UserConstructionScript`)
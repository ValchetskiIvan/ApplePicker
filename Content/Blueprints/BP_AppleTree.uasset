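; BP_AppleTree is a tree actor that moves back and forth along X while dropping apples.
; A looping half-second timer started on BeginPlay spawns a BP_Apple at the tree's location.
; Each Tick applies a randomized local X offset scaled by Direction, which flips whenever world X leaves the bounds.
; Those bounds come directly from the viewport's pixel width, used as plus or minus world units.
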(event `self.ReceiveBeginPlay`
  (set `self.WindowSize` (`WidgetLayoutLibrary.GetViewportSize`))
  (`KismetSystemLibrary.K2_SetTimerDelegate` (delegate `SpawnAppleEvent`) 0.5 true))

(event `SpawnAppleEvent`
  (`self.SpawnApple`))

(event `self.ReceiveTick`
  (params (DeltaSeconds :type "Float (single-precision)"))
  ;[1 1 1] Tree Movement
  (bind _isinzone (`self.InZoneCheck`))
  (if (not _isinzone)
    (`self.ChangeDirection` (`self.Direction`)))
  (`self.GenerateRandomVelocity`)
  (`self.K2_AddActorLocalOffset` (`KismetMathLibrary.MakeVector` (`self.Velocity`))))

(fn `ChangeDirection`
  (params (Direction :type Integer))
  (set `self.Direction` (* Direction -1)))

(fn `GenerateRandomVelocity`
  (set `self.Velocity` (* (`self.Direction`) (`KismetMathLibrary.RandomFloatInRange` 10.0 20.0))))

(fn `InZoneCheck`
  (returns (IsInZone :type Boolean))
  (bind _returnvalue_x (`KismetMathLibrary.BreakVector` (`self.K2_GetActorLocation`)))
  (bind _windowsize_x (`KismetMathLibrary.BreakVector2D` (`self.WindowSize`)))
  (return (and (< _returnvalue_x _windowsize_x) (> _returnvalue_x (* _windowsize_x -1.0)))))

(fn `SpawnApple`
  (bind (_returnvalue_x _returnvalue_y _returnvalue_z) (`KismetMathLibrary.BreakVector` (`self.K2_GetActorLocation`)))
  (`|SpawnActorFromClass` "/Game/Blueprints/BP_Apple.BP_Apple_C" (`KismetMathLibrary.MakeTransform` (`KismetMathLibrary.MakeVector` _returnvalue_x _returnvalue_y _returnvalue_z)) "Undefined" "OverrideRootScale" null null))

(fn `UserConstructionScript`)
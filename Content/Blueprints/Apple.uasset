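; Apple is a falling pickup for a catch game that either scores in the player's bucket or costs a heart when missed.
; A sphere hit on PB_Bucket adds the APPLE value to its AppleCounter, plays a success sound and destroys the apple.
; An overlap with BP_DeadZone plays a failure sound, destroys the apple, then calls HideHearth on the player pawn bucket's HealthBar.
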(event `self.Sphere.OnComponentHit`
  (params (HitComponent :type "PrimitiveComponent Object Reference") (OtherActor :type "Actor Object Reference") (OtherComp :type "PrimitiveComponent Object Reference") (NormalImpulse :type "Vector Structure") (Hit :type "HitResult Structure (by ref)"))
  ;[1 1 1] Bucket collision check
  (bind _aspb_bucket (cast `/Game/Blueprints/PB_Bucket` OtherActor))
  (set `/Game/Blueprints/PB_Bucket.AppleCounter` (+ (`/Game/Blueprints/PB_Bucket.AppleCounter` _aspb_bucket) (`self.APPLE`)) _aspb_bucket)
  (`GameplayStatics.PlaySound2D` "/Engine/EditorSounds/Notifications/CompileSuccess.CompileSuccess" 1.0 1.0 0.0 null null)
  (`self.K2_DestroyActor`))

(event `self.Sphere.OnComponentBeginOverlap`
  (params (OverlappedComponent :type "PrimitiveComponent Object Reference") (OtherActor :type "Actor Object Reference") (OtherComp :type "PrimitiveComponent Object Reference") (OtherBodyIndex :type Integer) (bFromSweep :type Boolean) (SweepResult :type "HitResult Structure (by ref)"))
  ;[1 1 1] DeadZone collision check
  (cast `/Game/Blueprints/BP_DeadZone` OtherActor)
  (`GameplayStatics.PlaySound2D` "/Engine/EditorSounds/Notifications/CompileFailed.CompileFailed" 1.0 1.0 0.0 null null)
  (`self.K2_DestroyActor`)
  (`self.HideHearth`))

(fn `HideHearth`
  (bind _aspb_bucket (cast `/Game/Blueprints/PB_Bucket` (`GameplayStatics.GetPlayerPawn` 0)))
  (`/Game/Blueprints/UI_HealthBar.HideHearth` (`/Game/Blueprints/PB_Bucket.HealthBar` _aspb_bucket)))

(fn `UserConstructionScript`)
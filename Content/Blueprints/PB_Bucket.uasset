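; PB_Bucket is the player-controlled bucket, which appears to belong to an apple-catching game.
; The Move Bucket input axis slides the Bucket component along its local X axis, scaled by Speed, with sweep collision.
; BeginPlay creates a UI_HealthBar widget and adds it to the viewport.
; Tick prints AppleCounter on screen every frame, but nothing in this file changes that counter.
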(event `self.ReceiveTick`
  (params (DeltaSeconds :type "Float (single-precision)"))
  (`KismetSystemLibrary.PrintString` (`KismetStringLibrary.Conv_IntToString` (`self.AppleCounter`)) true true (struct :`G` 0.66 :`B` 1.0 :`A` 1.0) DeltaSeconds))

(event `InputAxis|Move Bucket`
  (params (AxisValue :type "Float (single-precision)"))
  ;[1 1 1] Bucket Movement Handle
  (`SceneComponent.K2_AddLocalOffset` (`self.Bucket`) (`KismetMathLibrary.MakeVector` (* AxisValue (`self.Speed`))) true false))

(event `InitHealthBar`
  ;[1 1 1] HealthBar setting
  (bind _returnvalue (`|GenericCreateObject` "/Game/Blueprints/UI_HealthBar.UI_HealthBar_C" (`GameplayStatics.GetPlayerController` 0)))
  (bind _output_get (set `self.HealthBar` _returnvalue))
  (if (not (`Widget.IsInViewport` _output_get))
    (`UserWidget.AddToViewport` _output_get 0)))

(event `self.ReceiveBeginPlay`
  ;[1 1 1] HealthBar initialization
  (`self.InitHealthBar`))

(fn `UserConstructionScript`)
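; AppleTree is an actor that moves back and forth along X while dropping Apple actors.
; A looping one-second timer spawns an Apple at the tree's location.
; Each Tick reverses direction outside X bounds taken from the viewport width, then applies a random-speed offset.
; The viewport pixel width serves directly as world-space bounds, and movement is per frame, not scaled by delta time.
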(event `self.ReceiveBeginPlay`
  (set `self.WindowSize` (`WidgetLayoutLibrary.GetViewportSize`))
  (`KismetSystemLibrary.K2_SetTimerDelegate` (delegate `SpawnAppleEvent`) 1.0 true))

(event `SpawnAppleEvent`
  (`self.SpawnApple`))

(event `self.ReceiveTick`
  (params (DeltaSeconds :type "Float (single-precision)"))
  ;[1 1 1] Tree Movement
  (`self.InZoneCheck`)
  (`self.SetVelocity`)
  (`self.K2_AddActorLocalOffset` (`KismetMathLibrary.MakeVector` (`self.Velocity`))))

(fn `ChangeDirection`
  (set `self.Direction` (* (`self.Direction`) -1)))

(fn `InZoneCheck`
  (bind _returnvalue_x (`KismetMathLibrary.BreakVector` (`self.K2_GetActorLocation`)))
  (bind _windowsize_x (`KismetMathLibrary.BreakVector2D` (`self.WindowSize`)))
  (set `self.IsInZone` (and (< _returnvalue_x _windowsize_x) (> _returnvalue_x (* _windowsize_x -1.0)))))

(fn `SetVelocity`
  (if (not (`self.IsInZone`))
    (`self.ChangeDirection`))
  (set `self.Velocity` (* (`self.Direction`) (`KismetMathLibrary.RandomFloatInRange` 2.0 10.0))))

(fn `SpawnApple`
  (bind (_returnvalue_x _returnvalue_y _returnvalue_z) (`KismetMathLibrary.BreakVector` (`self.K2_GetActorLocation`)))
  (`|SpawnActorFromClass` "/Game/Blueprints/Apple.Apple_C" (`KismetMathLibrary.MakeTransform` (`KismetMathLibrary.MakeVector` _returnvalue_x _returnvalue_y _returnvalue_z)) "Undefined" "OverrideRootScale" null null))

(fn `UserConstructionScript`)